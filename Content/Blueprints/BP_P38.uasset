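; BP_P38 is a player-flyable P-38 aircraft pawn that constantly flies forward while input steers it.
; Tick spins the left and right propellers and feeds movement input along the actor's forward vector, scaled by speed and frame time.
; Roll and Pitch axis events clamp their input and apply frame-time-scaled local rotation, so steering follows the plane's own orientation.
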(event EventTick
  (params (DeltaSeconds :type Float%20%28single-precision%29))
  (Utilities|FlowControl|Sequence
    (:then_0
      (CallFunction|RotatePropeller (Variables|Default|GetRight)))
    (:then_1
      (CallFunction|RotatePropeller (Variables|Default|GetLeft)))
    (:then_2
      (CallFunction|MoveForward))))

(event Input|AxisEvents|InputAxisRoll
  (params (AxisValue :type Float%20%28single-precision%29))
  (Transformation|AddActorLocalRotation (Math|Rotator|MakeRotator (* (Math|Float|Clamp(Float) AxisValue -1.0) (Variables|Speed|GetRollRotationSpeed) (Utilities|Time|GetWorldDeltaSeconds)) 0.0 0.0) false false))

(event Input|AxisEvents|InputAxisPitch
  (params (AxisValue :type Float%20%28single-precision%29))
  (Transformation|AddActorLocalRotation (Math|Rotator|MakeRotator 0.0 (* (Math|Float|Clamp(Float) AxisValue -1.0) (Variables|Speed|GetPitchRotationSpeed) (Utilities|Time|GetWorldDeltaSeconds)) 0.0) false false))

(fn ConstructionScript)

(fn RotatePropeller
  (params (At :type Static%20Mesh%20Component%20Object%20Reference))
  (Transformation|AddRelativeRotation At (Math|Rotator|MakeRotator (* (Variables|Speed|GetPropellerRotateSpeed) (Utilities|Time|GetWorldDeltaSeconds)) 0.0 0.0) false false))

(fn MoveForward
  (Pawn|Input|AddMovementInput (* (Transformation|GetActorForwardVector) (* (Variables|Speed|GetMoveSpeed) (Utilities|Time|GetWorldDeltaSeconds))) 1.0 false))